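; Player character Blueprint handling Enhanced Input for camera-yaw-relative movement, look, jump, crouch and a mid-air downward slam (Sag).
; Holding the display-name input shows the nickname widget component.
; Jumping adds higher-priority keyboard and controller Sag mapping contexts, and Sag launches the character straight down once per press.
; Landing removes those contexts, deferred until release if Sag is still held, using the EnableSag flag.
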(event Input|EnhancedActionEvents|EnhancedInputActionIA_Move
  (params (ActionValue :type Vector%202D%20Structure) (ElapsedSeconds :type Float%20%28double-precision%29) (TriggeredSeconds :type Float%20%28double-precision%29) (InputAction :type Input%20Action%20Object%20Reference :default "/Game/Inputs/Actions/base/IA_Move.IA_Move"))
  (bind _returnvalue (Pawn|GetControlRotation :!class /Script/Engine.Pawn))
  (bind _yaw (Math|Rotator|BreakRotator _returnvalue))
  (bind _returnvalue_2 (Math|Rotator|MakeRotator 0.0 0.0 _yaw))
  ;[1 1 1] 移动
  (:Triggered
    (Pawn|Input|AddMovementInput (Math|Vector|GetRightVector _returnvalue_2) (.x ActionValue) false)
    (Pawn|Input|AddMovementInput (Math|Vector|GetForwardVector _returnvalue_2) (.y ActionValue) false)))

(event Input|EnhancedActionEvents|EnhancedInputActionIA_Look
  (params (ActionValue :type Vector%202D%20Structure) (ElapsedSeconds :type Float%20%28double-precision%29) (TriggeredSeconds :type Float%20%28double-precision%29) (InputAction :type Input%20Action%20Object%20Reference :default "/Game/Inputs/Actions/base/IA_Look.IA_Look"))
  ;[1 1 1] 视角和转向
  (:Triggered
    (Utilities|FlowControl|Sequence
      (:then_0
        (Pawn|Input|AddControllerYawInput (.x ActionValue)))
      (:then_1
        (Pawn|Input|AddControllerPitchInput (.y ActionValue))))))

(event Input|EnhancedActionEvents|EnhancedInputActionIA_DisplayName
  (params (ActionValue :type Boolean) (ElapsedSeconds :type Float%20%28double-precision%29) (TriggeredSeconds :type Float%20%28double-precision%29) (InputAction :type Input%20Action%20Object%20Reference :default "/Game/Inputs/Actions/base/IA_DisplayName.IA_DisplayName"))
  (bind _widget (Variables|Default|GetWidget))
  ;[1 1 1] 显示玩家昵称 TODO:将屏幕内的玩家昵称都显示
  (:Started
    (Development|SetHiddeninGame _widget false false))
  (:Completed
    (Development|SetHiddeninGame _widget true false)))

(event Input|EnhancedActionEvents|EnhancedInputActionIA_Jump
  (params (ActionValue :type Boolean) (ElapsedSeconds :type Float%20%28double-precision%29) (TriggeredSeconds :type Float%20%28double-precision%29) (InputAction :type Input%20Action%20Object%20Reference :default "/Game/Inputs/Actions/base/IA_Jump.IA_Jump"))
  ;[1 1 1] 跳跃
  (:Started
    (Character|Jump))
  (:Completed
    (Character|StopJumping)))

(event Input|EnhancedActionEvents|EnhancedInputActionIA_Crouch
  (params (ActionValue :type Boolean) (ElapsedSeconds :type Float%20%28double-precision%29) (TriggeredSeconds :type Float%20%28double-precision%29) (InputAction :type Input%20Action%20Object%20Reference :default "/Game/Inputs/Actions/base/IA_Crouch.IA_Crouch"))
  ;[1 1 1] 蹲下
  (:Started
    (Character|Crouch))
  (:Completed
    (Character|UnCrouch)))

(event Input|EnhancedActionEvents|EnhancedInputActionIA_Sag
  (params (ActionValue :type Boolean) (ElapsedSeconds :type Float%20%28double-precision%29) (TriggeredSeconds :type Float%20%28double-precision%29) (InputAction :type Input%20Action%20Object%20Reference :default "/Game/Inputs/Actions/sag/IA_Sag.IA_Sag"))
  (bind _returnvalue (Pawn|GetController))
  (bind _as玩家控制器 (Utilities|Casting|CastToPlayerController _returnvalue))
  (bind _returnvalue_2 (PlayerController|LocalPlayerSubsystems|GetEnhancedInputLocalPlayerSubsystem _as玩家控制器))
  ;[1 1 1] 下坠
  (:Started
    (if (Variables|Default|GetEnableSag)
      (Variables|Default|SetEnableSag false)
      (Character|LaunchCharacter "0.000000,0.000000,-2000.000000" true true)))
  (:Completed
    (Variables|Default|SetEnableSag true)
    (if (AI|Components|NavMovement|IsMovingonGround (Variables|Character|GetCharacterMovement))
      (Input|RemoveMappingContext _returnvalue_2 "/Game/Inputs/Keyboard/IMC_KeyboardSag.IMC_KeyboardSag" "(bIgnoreAllPressedKeysUntilRelease=True,bForceImmediately=False)")
      (Input|RemoveMappingContext _returnvalue_2 "/Game/Inputs/Control/IMC_ControlSag.IMC_ControlSag" "(bIgnoreAllPressedKeysUntilRelease=True,bForceImmediately=False)"))))

(event EventOnLanded
  (params (Hit :type Hit%20Result%20Structure%20%28by%20ref%29))
  (bind _returnvalue (Pawn|GetController))
  (bind _as玩家控制器 (Utilities|Casting|CastToPlayerController _returnvalue))
  (bind _returnvalue_2 (PlayerController|LocalPlayerSubsystems|GetEnhancedInputLocalPlayerSubsystem _as玩家控制器))
  ;[1 1 1] 下坠
  (if (Variables|Default|GetEnableSag)
    (Input|RemoveMappingContext _returnvalue_2 "/Game/Inputs/Keyboard/IMC_KeyboardSag.IMC_KeyboardSag" "(bIgnoreAllPressedKeysUntilRelease=True,bForceImmediately=False)")
    (Input|RemoveMappingContext _returnvalue_2 "/Game/Inputs/Control/IMC_ControlSag.IMC_ControlSag" "(bIgnoreAllPressedKeysUntilRelease=True,bForceImmediately=False)")))

(event EventOnJumped
  (bind _returnvalue (Pawn|GetController))
  (bind _as玩家控制器 (Utilities|Casting|CastToPlayerController _returnvalue))
  (bind _returnvalue_2 (PlayerController|LocalPlayerSubsystems|GetEnhancedInputLocalPlayerSubsystem _as玩家控制器))
  ;[1 1 1] 下坠
  (Input|AddMappingContext _returnvalue_2 "/Game/Inputs/Keyboard/IMC_KeyboardSag.IMC_KeyboardSag" 1 "(bIgnoreAllPressedKeysUntilRelease=True,bForceImmediately=False)")
  (Input|AddMappingContext _returnvalue_2 "/Game/Inputs/Control/IMC_ControlSag.IMC_ControlSag" 1 "(bIgnoreAllPressedKeysUntilRelease=True,bForceImmediately=False)"))

(fn ConstructionScript)