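; Player controller that applies saved option settings at startup and handles the pause menu.
; On BeginPlay it adds keyboard and control Enhanced Input contexts, loads options from the GameInstance, then sets the FPS widget, sound-class volumes, material quality and remapped keys.
; Key remapping only touches bindings that differ from their defaults.
; The pause action toggles a lazily created menu, switching game pause, input mode and cursor visibility.
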(event Input|EnhancedActionEvents|EnhancedInputActionIA_PauseGame
  (params (ActionValue :type Boolean) (ElapsedSeconds :type Float%20%28double-precision%29) (TriggeredSeconds :type Float%20%28double-precision%29) (InputAction :type Input%20Action%20Object%20Reference :default "/Game/Inputs/Actions/base/IA_PauseGame.IA_PauseGame"))
  ;[1 1 1] 暂停菜单
  (:Started
    (if (Variables|Default|GetShowPause)
      (CallFunction|UnPauseGame)
      (else
        (CallFunction|PauseGame)))))

(event EventBeginPlay
  (bind _returnvalue (PlayerController|LocalPlayerSubsystems|GetEnhancedInputLocalPlayerSubsystem))
  (Utilities|FlowControl|Sequence
    (:then_0
      ;[1 1 1] 使用增强输入
      (Utilities|IsValid _returnvalue
        (:Is%20Valid
          (Input|AddMappingContext _returnvalue "/Game/Inputs/Keyboard/IMC_BaseKeyboard.IMC_BaseKeyboard" 0 "(bIgnoreAllPressedKeysUntilRelease=True,bForceImmediately=False)")
          (Input|AddMappingContext _returnvalue "/Game/Inputs/Control/IMC_BaseControl.IMC_BaseControl" 0 "(bIgnoreAllPressedKeysUntilRelease=True,bForceImmediately=False)"))))
    (:then_1
      ;[1 1 1] 加载保存的设置选项值
      (bind _optionsetting (Class|BPIGameInstance|LoadOptionSettingData(Message) (Game|GetGameInstance)))
      (Variables|Default|SetOption%20Setting _optionsetting))
    (:then_2
      ;[1 1 1] 设置中是否有开启FPS
      (if (Variables|/Game/Blueprints/Save/BP_OptionSetting_Save.BP_OptionSetting_Save_C|GetShowFPS (Variables|Default|GetOption%20Setting))
        (CallFunction|ShowFPS)
        (else
          (CallFunction|HideFPS))))
    (:then_3
      ;[1 1 1] 初始化声音,按键,材质质量
      (OptionSetting|InitSound)
      (OptionSetting|InitMaterialQualityLevel)
      (OptionSetting|InitInputAction))))

(event EventUnPauseGame
  (Widget|RemovefromParent (Variables|Default|GetPauseGameWidget))
  (Game|SetGamePaused false)
  (Input|SetInputModeGameOnly self false)
  (Variables|Default|SetbShowMouseCursor false)
  (Variables|Default|SetShowPause false))

(event EventShowFPS
  (Variables|Default|GetFPSWidget
    (:then
      _)
    (:else
      (bind _returnvalue (UserInterface|CreateWidget "/Game/Widgets/WB_GameFrame.WB_GameFrame_C"))
      (Variables|Default|SetFPSWidget _returnvalue)))
  (UserInterface|Viewport|AddtoViewport (Variables|Default|GetFPSWidget) 0))

(event EventPauseGame
  (Variables|Default|GetPauseGameWidget
    (:then
      _)
    (:else
      (bind _returnvalue (UserInterface|CreateWidget "/Game/Widgets/WB_PauseGame.WB_PauseGame_C"))
      (Variables|Default|SetPauseGameWidget _returnvalue)))
  (UserInterface|Viewport|AddtoViewport (Variables|Default|GetPauseGameWidget) 0)
  (Game|SetGamePaused true)
  (Input|SetInputModeGameandUI self (Variables|Default|GetPauseGameWidget) "DoNotLock" false false)
  (Variables|Default|SetbShowMouseCursor true)
  (Variables|Default|SetShowPause true))

(event EventHideFPS
  (bind _fpswidget (Variables|Default|GetFPSWidget)
    (:then
      (Widget|RemovefromParent _fpswidget))
    (:else)))

(fn ConstructionScript)

(fn InitSound
  (Audio|SetSoundMixClassOverride "/Game/Blueprints/Audio/SM_Default.SM_Default" "/Game/Blueprints/Audio/SC_MainAudio.SC_MainAudio" (/ (Variables|/Game/Blueprints/Save/BP_OptionSetting_Save.BP_OptionSetting_Save_C|GetMasterVolume (Variables|Default|GetOption%20Setting)) 1e+02) 1.0 0.0 true)
  (Audio|SetSoundMixClassOverride "/Game/Blueprints/Audio/SM_Default.SM_Default" "/Game/Blueprints/Audio/SC_GameAudio.SC_GameAudio" (/ (Variables|/Game/Blueprints/Save/BP_OptionSetting_Save.BP_OptionSetting_Save_C|GetGameVolume (Variables|Default|GetOption%20Setting)) 1e+02) 1.0 0.0 false)
  (Audio|SetSoundMixClassOverride "/Game/Blueprints/Audio/SM_Default.SM_Default" "/Game/Blueprints/Audio/SC_VoiceAudio.SC_VoiceAudio" (/ (Variables|/Game/Blueprints/Save/BP_OptionSetting_Save.BP_OptionSetting_Save_C|GetVoiceVolume (Variables|Default|GetOption%20Setting)) 1e+02) 1.0 0.0 false)
  (Audio|SetSoundMixClassOverride "/Game/Blueprints/Audio/SM_Default.SM_Default" "/Game/Blueprints/Audio/SC_BackgroundAudio.SC_BackgroundAudio" (/ (Variables|/Game/Blueprints/Save/BP_OptionSetting_Save.BP_OptionSetting_Save_C|GetBackgroundVolume (Variables|Default|GetOption%20Setting)) 1e+02) 1.0 0.0 false))

(fn InitMaterialQualityLevel
  (Development|ExecuteConsoleCommand (Utilities|String|BuildString(Integer) "" "r.MaterialQualityLevel " (Variables|/Game/Blueprints/Save/BP_OptionSetting_Save.BP_OptionSetting_Save_C|GetMaterialQualityLevel%20 (Variables|Default|GetOption%20Setting))) 0))

(fn InitInputAction
  (bind _option_setting (Variables|Default|GetOption%20Setting))
  (bind _playerinputmap (Variables|/Game/Blueprints/Save/BP_OptionSetting_Save.BP_OptionSetting_Save_C|GetPlayerInputMap _option_setting))
  (bind _keys (Utilities|Map|Keys _playerinputmap))
  (for _array_element _keys
    (if (not (== (.CurrentKey (Utilities|Struct|BreakStruct_InputMap_Value (.Value (Utilities|Map|Find _playerinputmap _array_element)))) (.DefaultKey (Utilities|Struct|BreakStruct_InputMap_Value (.Value (Utilities|Map|Find _playerinputmap _array_element))))))
      (CallFunction|ChangeKeyMappingbyStruct (.CurrentKey (Utilities|Struct|BreakStruct_InputMap_Value (.Value (Utilities|Map|Find _playerinputmap _array_element)))) (.DefaultKey (Utilities|Struct|BreakStruct_InputMap_Value (.Value (Utilities|Map|Find _playerinputmap _array_element)))) (.ControlBlocks (Utilities|Struct|BreakStruct_InputMap_Value (.Value (Utilities|Map|Find _playerinputmap _array_element))))))))